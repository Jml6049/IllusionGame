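; NoteOverlay is an actor Blueprint that toggles an on-screen note widget with the F key.
; BeginPlay gets the player controller through player state 0, enables input on the actor and creates the stored NoteUI widget.
; F adds or removes the widget based on IsToggled.
; Showing the note disables the actor's own input, which also cuts off the F handler that would hide it and re-enable input.
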(event `Key|F`
  (params (Key :type "Key Structure"))
  (bind _noteui_ref (`self.NoteUI_Ref`))
  (bind _keyboard (`self.Keyboard`))
  ;[1 1 1] Toggles Note Overlay
  (:`Pressed`
    (if (`self.isToggled`)
      (`Widget.RemoveFromParent` _noteui_ref)
      (set `self.isToggled` false)
      (`self.EnableInput` _keyboard)
      (else
        (`UserWidget.AddToViewport` _noteui_ref 0)
        (set `self.isToggled` true)
        (`self.DisableInput` _keyboard)))))

(event `self.ReceiveBeginPlay`
  (bind _output_get (set `self.Keyboard` (`PlayerState.GetPlayerController` (`GameplayStatics.GetPlayerState` 0))))
  (`self.EnableInput` _output_get)
  (bind _returnvalue (`|CreateWidget` "/Game/NoteUI.NoteUI_C"))
  (set `self.NoteUI_Ref` _returnvalue))

(fn `UserConstructionScript`)