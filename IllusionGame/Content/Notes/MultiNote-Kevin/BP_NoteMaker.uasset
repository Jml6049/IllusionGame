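; BP_NoteMaker is an interactable note actor that lets the player open and close a readable note.
; Overlapping the actor enables input and copies its Note value to the third-person character's NoteIndex.
; Interact calls a FlipFlop that alternately shows the NoteDisplay widget with a paper sound or removes it.
; The Box toggles an interact prompt for the player, and leaving the actor disables input and closes the note.
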(event `self.ReceiveBeginPlay`
  (bind _returnvalue (`|CreateWidget` "/Game/Interactible/InteractPromptUI.InteractPromptUI_C"))
  (set `self.NewVar` _returnvalue))

(event `Inter`
  (`/Engine/EditorBlueprintResources/StandardMacros.FlipFlop`
    (:`A`
      (bind _returnvalue (`|CreateWidget` "/Game/Notes/MultiNote-Kevin/NoteDisplay.NoteDisplay_C"))
      (`UserWidget.AddToViewport` _returnvalue 0)
      (`GameplayStatics.PlaySound2D` "/Game/Notes/paper.paper" 0.2 1.0 0.2 null null))
    (:`B`
      (`/Engine/EditorBlueprintResources/StandardMacros.IsValid` _returnvalue :!label _label
        (:`Is Valid`
          (`Widget.RemoveFromParent` _returnvalue))))))

(event `self.ReceiveActorBeginOverlap`
  (params (OtherActor :type "Actor Object Reference"))
  (`self.EnableInput` (`GameplayStatics.GetPlayerController` 0))
  (bind _asbp_third_person_character (cast `/Game/ThirdPerson/Blueprints/BP_ThirdPersonCharacter` (`GameplayStatics.GetPlayerCharacter` 0)))
  (set `/Game/ThirdPerson/Blueprints/BP_ThirdPersonCharacter.NoteIndex` (`self.Note`) _asbp_third_person_character))

(event `self.ReceiveActorEndOverlap`
  (params (OtherActor :type "Actor Object Reference"))
  (`self.DisableInput` null)
  (goto _label))

(event `self.Box.OnComponentBeginOverlap`
  (params (OverlappedComponent :type "PrimitiveComponent Object Reference") (OtherActor :type "Actor Object Reference") (OtherComp :type "PrimitiveComponent Object Reference") (OtherBodyIndex :type Integer) (bFromSweep :type Boolean) (SweepResult :type "HitResult Structure (by ref)"))
  (if (== (`GameplayStatics.GetPlayerCharacter` 0) OtherActor)
    (`UserWidget.AddToViewport` (`self.NewVar`) 99)))

(event `self.Box.OnComponentEndOverlap`
  (params (OverlappedComponent :type "PrimitiveComponent Object Reference") (OtherActor :type "Actor Object Reference") (OtherComp :type "PrimitiveComponent Object Reference") (OtherBodyIndex :type Integer))
  (if (== OtherActor (`GameplayStatics.GetPlayerCharacter` 0))
    (`Widget.RemoveFromParent` (`self.NewVar`))))

(fn `Interact`
  (params (Interactor :type "Character Object Reference"))
  (returns (Success :type Boolean))
  (`self.Inter`)
  (return true))

(fn `UserConstructionScript`)