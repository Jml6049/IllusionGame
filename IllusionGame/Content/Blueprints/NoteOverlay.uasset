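; NoteOverlay is an actor Blueprint that lets the player show and hide a note overlay with the F key.
; On BeginPlay it enables input from the player's controller and creates one NoteUI widget, keeping a reference to it.
; Each F press flips IsToggled, adding or removing that widget from the viewport.
; Player movement is disabled while the note is shown and returns to walking when it is hidden.
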(event `Key|F`
  (params (Key :type "Key Structure"))
  (bind _noteui_ref (`self.NoteUI_Ref`))
  ;[1 1 1] Toggles Note Overlay
  (:`Pressed`
    (if (`self.isToggled`)
      (`Widget.RemoveFromParent` _noteui_ref)
      (set `self.isToggled` false)
      (`CharacterMovementComponent.SetMovementMode` (`Character.CharacterMovement` (`GameplayStatics.GetPlayerCharacter` 0)) "MOVE_Walking" 0)
      (else
        (`UserWidget.AddToViewport` _noteui_ref 0)
        (set `self.isToggled` true)
        (`CharacterMovementComponent.DisableMovement` (`Character.CharacterMovement` (`GameplayStatics.GetPlayerCharacter` 0)))))))

(event `self.ReceiveBeginPlay`
  ;[1 1 1] Creates the Note
  (bind _output_get (set `self.Keyboard` (`PlayerState.GetPlayerController` (`GameplayStatics.GetPlayerState` 0))))
  (`self.EnableInput` _output_get)
  (bind _returnvalue (`|CreateWidget` "/Game/NoteUI.NoteUI_C"))
  (set `self.NoteUI_Ref` _returnvalue))

(fn `UserConstructionScript`)