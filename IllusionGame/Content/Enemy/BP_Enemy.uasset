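; BP_Enemy is an AI enemy that chases the player on sight and ends the game on contact.
; Pawn sensing caches the player and starts AIMoveTo, with a five-second retriggerable delay clearing the sight flag.
; While unaware, Tick uses random delays to move it near a hardcoded point, then sets a fixed rotation.
; Box overlap with the cached player plays a jumpscare sound and shows the Game Over menu with UI-only input.
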(event `self.Box.OnComponentBeginOverlap`
  (params (OverlappedComponent :type "PrimitiveComponent Object Reference") (OtherActor :type "Actor Object Reference") (OtherComp :type "PrimitiveComponent Object Reference") (OtherBodyIndex :type Integer) (bFromSweep :type Boolean) (SweepResult :type "HitResult Structure (by ref)"))
  (bind _returnvalue (`GameplayStatics.GetPlayerController` 0))
  (if (== OtherActor (stale `self.PawnSensing.OnSeePawn` _asbp_third_person_character))
    (`GameplayStatics.PlaySound2D` "/Game/Enemy/jumpscareIllusionGame.jumpscareIllusionGame" 0.2 1.0 1.0 null null)
    (bind _returnvalue_2 (`|CreateWidget` "/Game/UI/GameOver_Menu.GameOver_Menu_C" _returnvalue))
    (`UserWidget.AddToViewport` _returnvalue_2 1100000)
    (set `PlayerController.bShowMouseCursor` true _returnvalue)
    (`WidgetBlueprintLibrary.SetInputMode_UIOnlyEx` _returnvalue _returnvalue_2 "DoNotLock" true)))

(event `self.ReceiveTick`
  (params (DeltaSeconds :type "Float (single-precision)"))
  (if (not (`self.canSeePlayer`))
    (`KismetSystemLibrary.Delay` (`KismetMathLibrary.RandomFloatInRange` 2.0 5.0))
    (`|AIMoveTo` self (`NavigationSystemV1.K2_GetRandomReachablePointInRadius` (664.030803 2264.140133 89.129343) 100.0 null null) null
      (:`OnSuccess`
        (`self.K2_SetActorRotation` (struct :`Yaw` 279.999998))))))

(event `self.PawnSensing.OnSeePawn`
  (params (Pawn :type "Pawn Object Reference"))
  (bind _asbp_third_person_character (cast `/Game/ThirdPerson/Blueprints/BP_ThirdPersonCharacter` Pawn))
  (`|ExecutionSequence`
    (:`then_0`
      (set `self.canSeePlayer` true)
      (`|AIMoveTo` self (0.0 0.0 0.0) _asbp_third_person_character))
    (:`then_1`
      (`KismetSystemLibrary.RetriggerableDelay` 5.0)
      (set `self.canSeePlayer` false))))

(fn `UserConstructionScript`)