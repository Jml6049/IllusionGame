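; BP_NoteMaker is an interactable world actor that shows and hides a note on screen.
; On overlap it enables input and copies its Note value into the third-person character's NoteIndex, presumably selecting which note displays.
; Interact fires a FlipFlop that alternately creates a NoteDisplay widget and removes it.
; Ending the overlap disables input and removes any open widget, without resetting the FlipFlop.
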(event `Inter`
  (`/Engine/EditorBlueprintResources/StandardMacros.FlipFlop`
    (:`A`
      (bind _returnvalue (`|CreateWidget` "/Game/Notes/MultiNote-Kevin/NoteDisplay.NoteDisplay_C"))
      (`UserWidget.AddToViewport` _returnvalue 0))
    (:`B`
      (`/Engine/EditorBlueprintResources/StandardMacros.IsValid` _returnvalue :!label _label
        (:`Is Valid`
          (`Widget.RemoveFromParent` _returnvalue))))))

(event `self.ReceiveActorBeginOverlap`
  (params (OtherActor :type "Actor Object Reference"))
  (`self.EnableInput` (`GameplayStatics.GetPlayerController` 0))
  (bind _asbp_third_person_character (cast `/Game/ThirdPerson/Blueprints/BP_ThirdPersonCharacter` (`GameplayStatics.GetPlayerCharacter` 0)))
  (set `/Game/ThirdPerson/Blueprints/BP_ThirdPersonCharacter.NoteIndex` (`self.Note`) _asbp_third_person_character))

(event `self.ReceiveActorEndOverlap`
  (params (OtherActor :type "Actor Object Reference"))
  (`self.DisableInput` null)
  (goto _label))

(fn `Interact`
  (params (Interactor :type "Character Object Reference"))
  (returns (Success :type Boolean))
  (`self.Inter`)
  (return true))

(fn `UserConstructionScript`)